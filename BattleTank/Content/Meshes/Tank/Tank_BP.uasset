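; Tank Blueprint that lets input axes turn the camera rig and aim the turret and barrel together.
; On BeginPlay it passes its Barrel component to SetBarrelReference.
; The azimuth axis yaws both the camera gimbal and the turret, while the attitude axis pitches both the spring arm and the barrel.
; Raw axis values feed local rotations directly, with no clamping or delta-time scaling.
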(event EventBeginPlay
  (Class|Tank|SetBarrelReference (Variables|Default|GetBarrel)))

(event Collision|EventActorBeginOverlap
  (params (OtherActor :type Actor%20Object%20Reference)))

(event EventTick
  (params (DeltaSeconds :type Float%20%28single-precision%29)))

(event Input|AxisEvents|InputAxisAzimuthBinding
  (params (AxisValue :type Float%20%28single-precision%29))
  ;[1 1 1] Camera and Turret orientation binding
  (Transformation|AddLocalRotation (Variables|Default|GetAzimuthGimbal) (Math|Rotator|MakeRotator 0.0 0.0 AxisValue) false false)
  (Transformation|AddLocalRotation (Variables|Default|GetTurret) (Math|Rotator|MakeRotator 0.0 0.0 AxisValue) false false))

(event Input|AxisEvents|InputAxisAttitudeBinding
  (params (AxisValue :type Float%20%28single-precision%29))
  ;[1 1 1] Camera and Turret orientation binding
  (Transformation|AddLocalRotation (Variables|Default|GetSpringArm) (Math|Rotator|MakeRotator 0.0 AxisValue 0.0) false false)
  (Transformation|AddLocalRotation (Variables|Default|GetBarrel) (Math|Rotator|MakeRotator 0.0 AxisValue 0.0) false false))

(fn ConstructionScript)